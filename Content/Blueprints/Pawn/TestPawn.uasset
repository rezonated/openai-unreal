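; TestPawn is a demo pawn that runs a chat-style AI conversation through a completion request, framed as a random stranger in a chat room.
; On BeginPlay it creates the WBP_ChatGPTDemo widget, switches input to UI only and hands itself to the widget.
; SendPrompt appends each prompt and reply to a growing Q/A instruction string as conversation history, shows the response in the widget and re-enables user input afterwards.
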(event Custom|SendPrompt
  (params (Prompt :type String) (CompletionModel :type ECompletionModel%20Enum :default "ECM_Davinci"))
  (bind _demowidget (Variables|Default|GetDemoWidget))
  (bind _output_get (Variables|Default|SetInstructions (Utilities|String|Append (Variables|Default|GetInstructions) Prompt " 
A: ")))
  (bind _response (|Completion _output_get CompletionModel)
    (:OnCompletionRequestComplete
      (Default|AddAIResponse _demowidget (.text (.choices _response)))
      (Default|ToggleUserInput (Variables|Default|GetDemoWidget) true)
      (Variables|Default|SetInstructions (Utilities|String|Append (Variables|Default|GetInstructions) (.text (.choices _response)) " 
Q: ")))
    (:OnCompletionRequestFailed
      (Default|ToggleUserInput _demowidget true))))

(event EventBeginPlay
  (Variables|Default|SetInstructions "Act as a random stranger in a chat room and reply to the questions.  
Q:")
  (bind _returnvalue (UserInterface|CreateWidget "/UnrealOpenAI/Blueprints/Widget/WBP_ChatGPTDemo.WBP_ChatGPTDemo_C" (Game|GetPlayerController 0)))
  (bind _output_get (Variables|Default|SetDemoWidget _returnvalue))
  (UserInterface|Viewport|AddtoViewport _output_get 0)
  (Input|SetInputModeUIOnly (Game|GetPlayerController 0) 0 "DoNotLock" true)
  (Variables|/UnrealOpenAI/Blueprints/Widget/WBP_ChatGPTDemo.WBP_ChatGPTDemo_C|SetTestPawn (Variables|Default|GetDemoWidget) self))

(fn ConstructionScript)

(fn NewFunction
  (params (NewParam :type AR%20Filter%20Structure)))